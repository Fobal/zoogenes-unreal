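; Blueprint function library that resolves ZooGene attributes, stored as trait type and value entries, into materials.
; GetZooGeneAttribute matches an enum's string against each trait type, returning its value and index, or -1 if absent.
; GetZooGeneMaterial appends a suffix to that value, finds the resulting slot name and returns the material at the same index in a parallel list.
; An unmatched slot name prints an error but still indexes the list.
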(fn `GetZooGeneAttribute`
  (params (AttributeArray :type "Array of /ZooGenesPlugin/Structures/S_ZooGenesAttributes Structure") (AttributeToFind :type "/ZooGenesPlugin/Enums/E_ZooGenesAttributes Enum" :default "NewEnumerator0"))
  (returns (ArrayElementValue :type String) (ArrayIndex :type Integer))
  (for (_array_element _array_index) AttributeArray
    (if (`KismetStringLibrary.EqualEqual_StrStr` (`|GetEnumeratorNameAsString` AttributeToFind) (break `/ZooGenesPlugin/Structures/S_ZooGenesAttributes` _array_element))
      (return (`.value_9_9FA550AB48CC2389CB7357AA410F96F9` (break `/ZooGenesPlugin/Structures/S_ZooGenesAttributes` _array_element)) _array_index)))
  (return "" -1))

(fn `GetZooGeneMaterial`
  (params (S_ZooGenes :type "/ZooGenesPlugin/Structures/S_ZooGenes Structure (by ref)") (AttributeToFind :type "/ZooGenesPlugin/Enums/E_ZooGenesAttributes Enum" :default "NewEnumerator0") (MaterialSlotNamePartB :type String) (MaterialsList :type "Array of MaterialInterface Object Reference") (MaterialSlotNamesList :type "Array of Name (by ref)"))
  (returns (MaterialListIndex :type Integer) (AttributeMaterial :type "MaterialInterface Object Reference") (AttributeArrayIndex :type Integer))
  (bind (_arrayelementvalue _arrayindex) (`self.GetZooGeneAttribute` (`.attributes_88_953544544DECFB085AEDE39E50CD9331` (break `/ZooGenesPlugin/Structures/S_ZooGenes` S_ZooGenes)) AttributeToFind))
  (if (== _arrayindex -1)
    (return -1 null -1)
    (else
      (bind _returnvalue (`KismetArrayLibrary.Array_Find` MaterialSlotNamesList (`KismetStringLibrary.Conv_StringToName` (`KismetStringLibrary.Concat_StrStr` _arrayelementvalue MaterialSlotNamePartB))))
      (if (== _returnvalue -1)
        (`KismetSystemLibrary.PrintString` null "Error: Trait not found"))
      (return _returnvalue (`|GetArrayItem` MaterialsList _returnvalue) _arrayindex))))