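; ZooGene character Blueprint that dresses one mesh in a named style from DT_ZooGenesList, starting with TigerStripes.
; BeginPlay caches the mesh's slot names and materials, then sets every slot to MT_Empty.
; UpdateZoogeneStyle clears the slots, then restores cached costume, headgear, accessory and body materials into slots matched by attribute-derived names.
; Data tables supply the facial expression material and, for ghosts, a replacement body material.
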(event `self.ReceiveBeginPlay`
  ;[0 0 0] Cache the material names in the start
  (`self.CacheZoogeneMaterialNames`)
  ;[0 0 0] Set TigerStripes as the initial ZooGene
  (`self.UpdateZoogeneStyle` "TigerStripes"))

(fn `CacheZoogeneMaterialNames`
  (set `self.MaterialSlotNamesCache` (`MeshComponent.GetMaterialSlotNames` (`self.Mesh`)))
  (`|ExecutionSequence`
    (:`then_0`
      (for _index (range 136)
        (`KismetArrayLibrary.Array_Add` (`self.MaterialsListCache`) (`PrimitiveComponent.GetMaterial` (`self.Mesh`) _index))))
    (:`then_1`
      (`self.ClearMaterials`))))

(fn `ClearMaterials`
  (for _index (range 136)
    (`PrimitiveComponent.SetMaterial` (`self.Mesh`) _index "/ZooGenesPlugin/Character/CharacterMaterials/MT_Empty.MT_Empty")))

(fn `UpdateZoogeneStyle`
  (params (ZooGeneName :type Name))
  (bind ((`imageUrl_93_C509231343DFC187BC6DE18721239D5D` _imageurl) (`attributes_88_953544544DECFB085AEDE39E50CD9331` _attributes)) (break `/ZooGenesPlugin/Structures/S_ZooGenes` (`self.SelectedZooGene`)))
  (bind _returnvalue (`|GetDataTableRow` "/ZooGenesPlugin/DataTables/DT_ZooGenesList.DT_ZooGenesList" ZooGeneName)
    (:`then`
      (set `self.SelectedZooGene` _returnvalue)
      (`self.ClearMaterials`)
      (`|ExecutionSequence`
        (:`then_0`
          ;[0 0 0] Facial
          (bind _arrayelementvalue (`/ZooGenesPlugin/Blueprints/BFL_ZooGene.GetZooGeneAttribute` _attributes "NewEnumerator6"))
          (bind _arrayelementvalue_2 (`/ZooGenesPlugin/Blueprints/BFL_ZooGene.GetZooGeneAttribute` _attributes "NewEnumerator5"))
          (bind _returnvalue_2 (`|GetDataTableRow` "/ZooGenesPlugin/DataTables/DT_ZooGenesFacial.DT_ZooGenesFacial" (`KismetStringLibrary.Conv_StringToName` _arrayelementvalue))
            (:`then`
              (`PrimitiveComponent.SetMaterial` (`self.Mesh`) (`KismetArrayLibrary.Array_Find` (`self.MaterialSlotNamesCache`) (`KismetStringLibrary.Conv_StringToName` (`KismetStringLibrary.Concat_StrStr` _arrayelementvalue_2 "_facial_MT"))) (`.Expression_MT_8_0B655BEF4969381A6D2962BC41FDA909` (break `/ZooGenesPlugin/Structures/S_ZooGenesFacial` _returnvalue_2))))))
        (:`then_1`
          ;[0 0 0] Costume
          (bind (_materiallistindex _attributematerial) (`/ZooGenesPlugin/Blueprints/BFL_ZooGene.GetZooGeneMaterial` (`self.SelectedZooGene`) "NewEnumerator2" "_MT" (`self.MaterialsListCache`) (`self.MaterialSlotNamesCache`)))
          (`PrimitiveComponent.SetMaterial` (`self.Mesh`) _materiallistindex _attributematerial))
        (:`then_2`
          ;[0 0 0] Headgear
          (bind (_materiallistindex_2 _attributematerial_2) (`/ZooGenesPlugin/Blueprints/BFL_ZooGene.GetZooGeneMaterial` (`self.SelectedZooGene`) "NewEnumerator0" "_MT" (`self.MaterialsListCache`) (`self.MaterialSlotNamesCache`)))
          (`PrimitiveComponent.SetMaterial` (`self.Mesh`) _materiallistindex_2 _attributematerial_2))
        (:`then_3`
          ;[0 0 0] Accessory
          (bind (_materiallistindex_3 _attributematerial_3) (`/ZooGenesPlugin/Blueprints/BFL_ZooGene.GetZooGeneMaterial` (`self.SelectedZooGene`) "NewEnumerator1" "_MT" (`self.MaterialsListCache`) (`self.MaterialSlotNamesCache`)))
          (`PrimitiveComponent.SetMaterial` (`self.Mesh`) _materiallistindex_3 _attributematerial_3))
        (:`then_4`
          ;[0 0 0] Ghost
          (bind _arrayelementvalue_3 (`/ZooGenesPlugin/Blueprints/BFL_ZooGene.GetZooGeneAttribute` (`.attributes_88_953544544DECFB085AEDE39E50CD9331` (break `/ZooGenesPlugin/Structures/S_ZooGenes` (`self.SelectedZooGene`))) "NewEnumerator7"))
          (if (`KismetStringLibrary.EqualEqual_StrStr` _arrayelementvalue_3 "Yes")
            (bind _arrayelementvalue_4 (`/ZooGenesPlugin/Blueprints/BFL_ZooGene.GetZooGeneAttribute` (`.attributes_88_953544544DECFB085AEDE39E50CD9331` (break `/ZooGenesPlugin/Structures/S_ZooGenes` (`self.SelectedZooGene`))) "NewEnumerator5"))
            (bind _returnvalue_3 (`|GetDataTableRow` "/ZooGenesPlugin/DataTables/DT_ZooGeneGhosts.DT_ZooGeneGhosts" (`KismetStringLibrary.Conv_StringToName` (`KismetStringLibrary.ToLower` _arrayelementvalue_4)))
              (:`then`
                (bind _materiallistindex_4 (`/ZooGenesPlugin/Blueprints/BFL_ZooGene.GetZooGeneMaterial` (`self.SelectedZooGene`) "NewEnumerator5" "_body_MT" (`self.MaterialsListCache`) (`self.MaterialSlotNamesCache`)))
                (`PrimitiveComponent.SetMaterial` (`self.Mesh`) _materiallistindex_4 (break `/ZooGenesPlugin/Structures/S_ZooGenesGhosts` _returnvalue_3))))
            (else
              (bind (_materiallistindex_5 _attributematerial_4) (`/ZooGenesPlugin/Blueprints/BFL_ZooGene.GetZooGeneMaterial` (`self.SelectedZooGene`) "NewEnumerator5" "_body_MT" (`self.MaterialsListCache`) (`self.MaterialSlotNamesCache`)))
              (`PrimitiveComponent.SetMaterial` (`self.Mesh`) _materiallistindex_5 _attributematerial_4))))))))

(fn `UserConstructionScript`)